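; Snowday HUD Blueprint that creates and manages the start screen, pause screen and in-game player HUD widgets.
; BeginPlay adds all three to the viewport and switches to UI-only input with a cursor, focused on the start screen.
; Start and Continue button bindings pair with StartGame and UnpauseGame, which dismiss their screen, then share logic restoring game input, showing the HUD and unpausing.
; Nothing here pauses the game or reveals the pause screen.
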(event `self.ReceiveBeginPlay`
  (bind _returnvalue (`GameplayStatics.GetPlayerController` 0))
  (`self.SpawnStartScreen`)
  (`WidgetBlueprintLibrary.SetInputMode_UIOnlyEx` _returnvalue (`self.StartScreen`))
  (set `PlayerController.bShowMouseCursor` true _returnvalue)
  (`self.SpawnPauseScreen`)
  (`self.SpawnPlayerHUD`))

(event `StartGame`
  (bind _returnvalue (`GameplayStatics.GetPlayerController` 0))
  (`Widget.RemoveFromParent` (`self.StartScreen`))
  (`WidgetBlueprintLibrary.SetInputMode_GameOnly` _returnvalue true :!label _label)
  (set `PlayerController.bShowMouseCursor` false _returnvalue)
  (`Widget.SetVisibility` (`self.PlayerHUD`) "HitTestInvisible")
  (`GameplayStatics.SetGamePaused` false))

(event `UnpauseGame`
  (`Widget.SetVisibility` (`self.PauseScreen`) "Hidden")
  (goto _label))

(fn `SpawnPauseScreen`
  (bind _returnvalue (`|CreateWidget` "/Game/Snowday/Blueprints/UI/WBP_PauseScreen.WBP_PauseScreen_C"))
  (bind _output_get (set `self.PauseScreen` _returnvalue))
  (add `/Game/Snowday/Blueprints/UI/WBP_PauseScreen.ContinueButtonClicked` _output_get (`|CreateDelegate` :!event `UnpauseGame`))
  (`UserWidget.AddToViewport` _output_get 0))

(fn `SpawnPlayerHUD`
  (bind _returnvalue (`|CreateWidget` "/Game/Snowday/Blueprints/UI/WBP_PlayerHUD.WBP_PlayerHUD_C"))
  (bind _output_get (set `self.PlayerHUD` _returnvalue))
  (`UserWidget.AddToViewport` _output_get 0))

(fn `SpawnStartScreen`
  (bind _returnvalue (`|CreateWidget` "/Game/Snowday/Blueprints/UI/WBP_StartScreen.WBP_StartScreen_C"))
  (bind _output_get (set `self.StartScreen` _returnvalue))
  (add `/Game/Snowday/Blueprints/UI/WBP_StartScreen.StartButtonClicked` _output_get (`|CreateDelegate` :!event `StartGame`))
  (`UserWidget.AddToViewport` _output_get 0))

(fn `UserConstructionScript`)