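; BP_SnowTriggerBox is a one-shot trigger volume that notifies the first overlapping actor about flattened snow.
; On overlap it sends FlattenedSnowMessage with its SnowGainRate to that actor, marks itself flattened, and optionally destroys itself.
; With debug enabled, it draws its collision component's bounds as a box every tick.
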(event `self.ReceiveActorBeginOverlap`
  (params (OtherActor :type "Actor Object Reference"))
  (if (not (`self.IsFlattened`))
    (message `/Game/Snowday/Blueprints/Interfaces/BPI_SnowTriggers.FlattenedSnow` OtherActor (`self.SnowGainRate`))
    (set `self.IsFlattened` true)
    (if (`self.DestroyOnEnter`)
      (`self.K2_DestroyActor`))))

(event `self.ReceiveTick`
  (params (DeltaSeconds :type "Float (single-precision)"))
  (bind (_origin _boxextent) (`KismetSystemLibrary.GetComponentBounds` (`self.CollisionComponent`)))
  (if (`self.EnableDebug`)
    (`KismetSystemLibrary.DrawDebugBox` _origin _boxextent (struct :`R` 0.781753 :`B` 1.0 :`A` 1.0) (struct) 0.0 5.0)))

(fn `UserConstructionScript`)