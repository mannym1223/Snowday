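; BP_SnowPathTriggerSpawner tiles the area of its Plane component with a grid of BP_SnowTriggerBox actors at BeginPlay.
; It derives cell size and first cell center from the plane's bounds, dividing both axes by Rows.
; Nested Rows and Columns loops spawn each box at world Z zero.
; Each box's X and Y scale is adjusted from its colliding bounds to fit one cell.
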(event `self.ReceiveBeginPlay`
  (bind (_origin _boxextent) (`KismetSystemLibrary.GetComponentBounds` (`self.Plane`)))
  (bind (_returnvalue_x _returnvalue_y) (`KismetMathLibrary.BreakVector` (/ (* _boxextent 2.0) (`self.Rows`))))
  (set `self.BoxSizeX` _returnvalue_x)
  (set `self.BoxSizeY` _returnvalue_y)
  (set `self.StartPointX` (+ (/ _returnvalue_x 2.0) (.x (- _origin _boxextent)))) ; start point with offset
  (set `self.StartPointY` (+ (/ _returnvalue_y 2.0) (.y (- _origin _boxextent))))
  (for _index (range (`self.Rows`))
    (for _index_2 (range (`self.Columns`))
      (bind _returnvalue (`|SpawnActorFromClass` "/Game/Snowday/Blueprints/Environment/BP_SnowTriggerBox.BP_SnowTriggerBox_C" (`KismetMathLibrary.MakeTransform` (`KismetMathLibrary.MakeVector` (+ (* _index (`self.BoxSizeX`)) (`self.StartPointX`)) (+ (* _index_2 (`self.BoxSizeY`)) (`self.StartPointY`)))) "AlwaysSpawn" "OverrideRootScale" self null))
      (bind (_returnvalue_x_2 _returnvalue_y_2 _returnvalue_z) (`KismetMathLibrary.BreakVector` (`self.GetActorScale3D` _returnvalue)))
      ;[1 1 1] Scale trigger box to match correct size of rows/columns
      (`self.SetActorScale3D` _returnvalue (`KismetMathLibrary.MakeVector` (* (/ (`self.BoxSizeX`) (.x (* (`.BoxExtent` (`self.GetActorBounds` _returnvalue true true)) 2.0))) _returnvalue_x_2) (* (/ (`self.BoxSizeY`) (.y (* (`.BoxExtent` (`self.GetActorBounds` _returnvalue true true)) 2.0))) _returnvalue_y_2) _returnvalue_z)))))

(fn `UserConstructionScript`)