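; Snowball pawn that grows as it flattens snow, using its sphere collider radius as the snow amount.
; FlattenedSnow adds to the collider's scale, updates the current radius, calls SnowChanged and triggers a zoom out.
; The zoom timeline incrementally lengthens the spring arm, scaled by ZoomRate.
; Getters expose current and maximum radius, though growth is not clamped to that maximum here.
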(event `self.ReceiveBeginPlay`
  (set `self.CurrentRadius` (`SphereComponent.GetScaledSphereRadius` (`self.SphereCollider`))))

(event `self.ReceiveTick`
  (params (DeltaSeconds :type "Float (single-precision)")))

(event `/Game/Snowday/Blueprints/Interfaces/BPI_SnowTriggers.FlattenedSnow`
  (params (`In Snow Amount` :type "Float (double-precision)"))
  (bind _spherecollider (`self.SphereCollider`))
  (`SceneComponent.SetRelativeScale3D` _spherecollider (+ (`SceneComponent.RelativeScale3D` _spherecollider) `In Snow Amount`))
  (set `self.CurrentRadius` (`SphereComponent.GetScaledSphereRadius` (`self.SphereCollider`)))
  (`self.SnowChanged`)
  (`self.ZoomOut`))

(event `ZoomOut`
  (bind _springarm (`self.SpringArm`))
  (bind (_direction _linearzoom) (`Timeline|TL_Zoom` :!via `PlayFromStart`)
    (:`Update`
      (set `SpringArmComponent.TargetArmLength` (+ (`SpringArmComponent.TargetArmLength` _springarm) (* _linearzoom (`self.ZoomRate`))) _springarm))))

(fn `GetMaxSnow`
  (returns (MaxSnow :type "Float (double-precision)"))
  (return (`self.MaxRadius`)))

(fn `GetSnowAmount`
  (returns (SnowAmount :type "Float (double-precision)"))
  (return (`self.CurrentRadius`)))

(fn `UserConstructionScript`)